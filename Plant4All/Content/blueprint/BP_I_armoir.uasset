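; BP_I_armoir is an interactable Blueprint, apparently an armoire, that opens and closes its own UI panel when interacted with.
; Each Interraction event alternates through a FlipFlop between creating a WBP_armoir widget on the viewport and removing it.
; Both branches also toggle the mouse cursor and the IsInUI flag on the first-person controller.
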(event EventInterraction
  (bind _asbp_first_person_player_controller (CallFunction|GetFirstPersonController))
  (bind _asbp_first_person_player_controller_2 (CallFunction|GetFirstPersonController))
  (Utilities|FlowControl|FlipFlop
    (:A
      (bind _returnvalue (UserInterface|CreateWidget "/Game/Widget/WBP_armoir.WBP_armoir_C"))
      (UserInterface|Viewport|AddtoViewport _returnvalue 0)
      (Variables|/Script/Engine.PlayerController|SetbShowMouseCursor _asbp_first_person_player_controller_2 true)
      (Variables|/Game/FirstPerson/Blueprints/BP_FirstPersonPlayerController.BP_FirstPersonPlayerController_C|SetisInUI _asbp_first_person_player_controller_2 true))
    (:B
      (Widget|RemovefromParent _returnvalue)
      (Variables|/Script/Engine.PlayerController|SetbShowMouseCursor _asbp_first_person_player_controller false)
      (Variables|/Game/FirstPerson/Blueprints/BP_FirstPersonPlayerController.BP_FirstPersonPlayerController_C|SetisInUI _asbp_first_person_player_controller false))))

(fn ConstructionScript
  (|CallParentFunction))