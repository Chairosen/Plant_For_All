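; A composter interactable that turns plants into fertilizer.
; On interaction, while it holds fewer than three plants and the first-person controller reports a plant, it removes that item and increments its count.
; Otherwise, once the count reaches three, it tries to add a fertilizer item to the controller and deducts three plants only if that add succeeds.
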(event EventInterraction
  (bind _asbp_first_person_player_controller (CallFunction|GetFirstPersonController))
  (if (and (Default|IsPlant (CallFunction|GetFirstPersonController)) (< (Variables|Default|GetnumberPlant) 3))
    (Default|RemoveItem _asbp_first_person_player_controller)
    (Variables|Default|SetnumberPlant (+ (Variables|Default|GetnumberPlant) 1))
    (elif (>= (Variables|Default|GetnumberPlant) 3)
      (bind _place (Default|AddItem _asbp_first_person_player_controller "/Game/data/DA_I_O_fertilizer.DA_I_O_fertilizer"))
      (if _place
        (Variables|Default|SetnumberPlant (+ (Variables|Default|GetnumberPlant) -3))))))

(fn ConstructionScript
  (|CallParentFunction))