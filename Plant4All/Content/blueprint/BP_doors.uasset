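; BP_doors is a pair of sliding doors that open and close as the first-person character enters or leaves the Captor trigger.
; Overlap begin and end each restart their own timeline, whose updates nudge RightDoor and LeftDoor in opposite X directions with sweep.
; Movement is a fixed relative step per update rather than an interpolated position, so travel depends on update count.
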(event OnComponentBeginOverlap(captor)
  (params (OverlappedComponent :type Primitive%20Component%20Object%20Reference) (OtherActor :type Actor%20Object%20Reference) (OtherComp :type Primitive%20Component%20Object%20Reference) (OtherBodyIndex :type Integer) (bFromSweep :type Boolean) (SweepResult :type Hit%20Result%20Structure%20%28by%20ref%29))
  (Utilities|Casting|CastToBP_FirstPersonCharacter OtherActor)
  (Timeline|Timeline PlayFromStart
    (:Update
      (Transformation|AddRelativeLocation (Variables|Default|GetrightDoor) (Math|Vector|MakeVector 1.0 0.0 0.0) true false)
      (Transformation|AddRelativeLocation (Variables|Default|GetleftDoor) (Math|Vector|MakeVector -1.0 0.0 0.0) true false))))

(event OnComponentEndOverlap(captor)
  (params (OverlappedComponent :type Primitive%20Component%20Object%20Reference) (OtherActor :type Actor%20Object%20Reference) (OtherComp :type Primitive%20Component%20Object%20Reference) (OtherBodyIndex :type Integer))
  (Utilities|Casting|CastToBP_FirstPersonCharacter OtherActor)
  (Timeline|Timeline_0 PlayFromStart
    (:Update
      (Transformation|AddRelativeLocation (Variables|Default|GetrightDoor) (Math|Vector|MakeVector -1.0 0.0 0.0) true false)
      (Transformation|AddRelativeLocation (Variables|Default|GetleftDoor) (Math|Vector|MakeVector 1.0 0.0 0.0) true false))))

(fn ConstructionScript)