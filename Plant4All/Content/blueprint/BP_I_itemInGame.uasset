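; BP_I_itemInGame is an interactable world item that the player can pick up and put back.
; On BeginPlay it applies the mesh from its Item data.
; Interraction toggles on Take: it either adds the item to the first-person controller and hides the mesh without collision, or, if that item is the controller's CurrentItem, removes it and restores the mesh.
; Cursor hover over the mesh sets the controller's Action flag.
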(event OnBeginCursorOver(StaticMesh1)
  (params (TouchedComponent :type Primitive%20Component%20Object%20Reference))
  (Variables|/Game/FirstPerson/Blueprints/BP_FirstPersonPlayerController.BP_FirstPersonPlayerController_C|Setaction (CallFunction|GetFirstPersonController) true))

(event OnEndCursorOver(StaticMesh1)
  (params (TouchedComponent :type Primitive%20Component%20Object%20Reference))
  (Variables|/Game/FirstPerson/Blueprints/BP_FirstPersonPlayerController.BP_FirstPersonPlayerController_C|Setaction (CallFunction|GetFirstPersonController) false))

(event EventBeginPlay
  (Components|StaticMesh|SetStaticMesh (Variables|Default|GetStaticMesh1) (Variables|/Game/blueprint/BP_DA_inventory.BP_DA_inventory_C|Getmesh (Variables|Default|Getitem))))

(event EventInterraction
  (bind _asbp_first_person_player_controller (CallFunction|GetFirstPersonController))
  (bind _staticmesh1 (Variables|Default|GetStaticMesh1))
  (bind _staticmesh1_2 (Variables|Default|GetStaticMesh1))
  (if (Variables|Default|Gettake)
    (if (== (Variables|/Game/FirstPerson/Blueprints/BP_FirstPersonPlayerController.BP_FirstPersonPlayerController_C|GetcurrentItem _asbp_first_person_player_controller) (Variables|Default|Getitem))
      (Default|RemoveItem _asbp_first_person_player_controller)
      (Rendering|SetVisibility _staticmesh1 true false)
      (Collision|SetCollisionEnabled _staticmesh1 "QueryAndPhysics")
      (Variables|Default|Settake false))
    (else
      (Default|AddItem (CallFunction|GetFirstPersonController) (Variables|Default|Getitem))
      (Rendering|SetVisibility _staticmesh1_2 false false)
      (Collision|SetCollisionEnabled _staticmesh1_2 "NoCollision")
      (Variables|Default|Settake true))))

(fn ConstructionScript
  (|CallParentFunction))