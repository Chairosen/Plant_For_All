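; Trapdoor actor with a temporary interaction that toggles a placeholder plant in its machine.
; When the first-person character begins overlapping the Machine component with IsInteract set, it spawns BP_Temp_Plant above the machine, or destroys one if IsOccupied.
; IsOccupied tracks the state, and removal uses GetActorOfClass rather than a stored reference, so it takes any plant found in the level.
; Debug prints report each outcome.
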(event OnComponentBeginOverlap(Machine)
  (params (OverlappedComponent :type Primitive%20Component%20Object%20Reference) (OtherActor :type Actor%20Object%20Reference) (OtherComp :type Primitive%20Component%20Object%20Reference) (OtherBodyIndex :type Integer) (bFromSweep :type Boolean) (SweepResult :type Hit%20Result%20Structure%20%28by%20ref%29))
  (bind _machine (Variables|Default|GetMachine))
  (bind _returnvalue (Transformation|GetWorldLocation _machine))
  ;[0.15 0.15 0.15 0.5] fais spawn la plante dans machine
  ;;[0.15 0.15 0.15 0.5] Interaction temporaire
  (Utilities|Casting|CastToBP_FirstPersonCharacter OtherActor)
  (if (Variables|Default|GetisInteract)
    (if (Variables|Default|GetisOccupied)
      (Development|PrintString "Occupied")
      (bind _returnvalue_2 (Actor|GetActorOfClass "/Game/blueprint/BP_Temp_Plant.BP_Temp_Plant_C"))
      (Actor|DestroyActor _returnvalue_2)
      (Development|PrintString "delete")
      (Variables|Default|SetisOccupied false)
      (else
        (bind _returnvalue_3 (Game|SpawnActorfromClass "/Game/blueprint/BP_Temp_Plant.BP_Temp_Plant_C" (Transformation|GetActorTransform) "Undefined" "MultiplyWithRoot" 0 0))
        (Transformation|SetActorLocation _returnvalue_3 (Math|Vector|MakeVector (.x _returnvalue) (.y _returnvalue) (+ (.z _returnvalue) 1e+02)) false false)
        (Development|PrintString "spawned")
        (Variables|Default|SetisOccupied true)
        (if true
          _)))
    (else
      (Development|PrintString "false"))))

(event Collision|EventActorBeginOverlap
  (params (OtherActor :type Actor%20Object%20Reference)))

(event EventTick
  (params (DeltaSeconds :type Float%20%28single-precision%29)))

(fn ConstructionScript)